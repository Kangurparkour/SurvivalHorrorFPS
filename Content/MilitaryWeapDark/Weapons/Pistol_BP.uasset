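; Pistol weapon actor with a Fire event that shoots while its ammo count is above zero.
; Each shot plays the fire animation on the skeletal mesh, spawns Ammo and Ammo2 actors at the AmmoEject and MuzzleFlash sockets respectively, then decrements the count.
; When out of ammo, Fire only plays the Pistol_Lower 2D sound; there is no reload logic.
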(event Custom|Fire
  (if (> (Variables|Default|GetAmmo) 0)
    (Components|Animation|PlayAnimation (Variables|Default|GetPistolSkeletarMesh) "/Game/MilitaryWeapDark/Weapons/Anims/Fire_Pistol_W.Fire_Pistol_W" false)
    (Game|SpawnActorfromClass "/Game/MilitaryWeapDark/Weapons/Ammo.Ammo_C" (Transformation|GetSocketTransform (Variables|Default|GetPistolSkeletarMesh) "AmmoEject" "RTS_World") "Undefined" 0 0)
    (Game|SpawnActorfromClass "/Game/MilitaryWeapDark/Weapons/Ammo2.Ammo2_C" (Transformation|GetSocketTransform (Variables|Default|GetPistolSkeletarMesh) "MuzzleFlash" "RTS_World") "Undefined" 0 0)
    (Variables|Default|SetAmmo (- (Variables|Default|GetAmmo) 1))
    (else
      (Audio|PlaySound2D "/Game/MilitaryWeapDark/Sound/Pistol/Wavs/Pistol_Lower.Pistol_Lower" 1.0 1.0 0.0 0 0))))

(event Collision|EventActorBeginOverlap
  (params (OtherActor :type Actor%20Object%20Reference)))

(event EventTick
  (params (DeltaSeconds :type Float%20%28single-precision%29)))

(fn ConstructionScript)