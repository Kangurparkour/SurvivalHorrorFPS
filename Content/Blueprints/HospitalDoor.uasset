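; HospitalDoor is a sliding door that opens when the player character enters its detection volume and closes when they leave.
; Opening calls CallPowerToMainDoor and then proceeds only if HasPower is true, while closing has no power check.
; A timeline played forward or in reverse at DoorSpeed lerps the door mesh along its relative Y axis.
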(event OnComponentBeginOverlap(PlayerDetector)
  (params (OverlappedComponent :type Primitive%20Component%20Object%20Reference) (OtherActor :type Actor%20Object%20Reference) (OtherComp :type Primitive%20Component%20Object%20Reference) (OtherBodyIndex :type Integer) (bFromSweep :type Boolean) (SweepResult :type Hit%20Result%20Structure%20%28by%20ref%29))
  (Utilities|Casting|CastToThirdPersonCharacter OtherActor)
  (CallFunction|OpenDoor))

(event OnComponentEndOverlap(PlayerDetector)
  (params (OverlappedComponent :type Primitive%20Component%20Object%20Reference) (OtherActor :type Actor%20Object%20Reference) (OtherComp :type Primitive%20Component%20Object%20Reference) (OtherBodyIndex :type Integer))
  (Utilities|Casting|CastToThirdPersonCharacter OtherActor)
  (CallFunction|CloseDoor))

(event Custom|CloseDoor
  (Components|Timeline|SetPlayRate (Variables|Default|GetDoorOpen) (Variables|Default|GetDoorSpeed))
  (bind _opendoortrack (Timeline|DoorOpen Reverse)
    (:Update
      (Transformation|SetRelativeLocation (Variables|Default|GetDoorMesh) (Math|Vector|MakeVector 0.0 (Math|Float|Lerp -1.5e+02 -4.3e+02 _opendoortrack) 0.0) false false))))

(event Custom|OpenDoor
  (Default|CallPowertoMainDoor)
  (if (Variables|Default|GetHasPower)
    (Components|Timeline|SetPlayRate (Variables|Default|GetDoorOpen) (Variables|Default|GetDoorSpeed))
    (bind _opendoortrack (Timeline|DoorOpen Play)
      (:Update
        (Transformation|SetRelativeLocation (Variables|Default|GetDoorMesh) (Math|Vector|MakeVector 0.0 (Math|Float|Lerp -1.5e+02 -4.3e+02 _opendoortrack) 0.0) false false)))))

(fn ConstructionScript)