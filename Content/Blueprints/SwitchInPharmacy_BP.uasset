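; A pharmacy lever switch Blueprint that the player toggles to give or cut power to a door.
; Overlapping Box1 as the ThirdPersonCharacter enables input, and the Action key then alternates through a FlipFlop.
; The Switching timeline plays or reverses to rotate the lever.
; On every timeline update, IsOff sets the light green and calls power on when true (despite its name), or red and power cut when false.
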(event OnComponentBeginOverlap(Box1)
  (params (OverlappedComponent :type Primitive%20Component%20Object%20Reference) (OtherActor :type Actor%20Object%20Reference) (OtherComp :type Primitive%20Component%20Object%20Reference) (OtherBodyIndex :type Integer) (bFromSweep :type Boolean) (SweepResult :type Hit%20Result%20Structure%20%28by%20ref%29))
  (Utilities|Casting|CastToThirdPersonCharacter OtherActor)
  (Variables|Default|SetisDetected true)
  (Input|EnableInput (Game|GetPlayerController 0)))

(event OnComponentEndOverlap(Box1)
  (params (OverlappedComponent :type Primitive%20Component%20Object%20Reference) (OtherActor :type Actor%20Object%20Reference) (OtherComp :type Primitive%20Component%20Object%20Reference) (OtherBodyIndex :type Integer))
  (Utilities|Casting|CastToThirdPersonCharacter OtherActor)
  (Variables|Default|SetisDetected false)
  (Input|DisableInput (Game|GetPlayerController 0)))

(event Input|ActionEvents|InputActionAction
  (params (Key :type Key%20Structure :default "None"))
  (:Pressed
    (if (Variables|Default|GetisDetected)
      (Components|Timeline|SetPlayRate (Variables|Default|Getswitching) 1.0)
      (Utilities|FlowControl|FlipFlop
        (:A
          (Variables|Default|SetIsOff true)
          (bind _newtrack_0 (Timeline|switching Play)
            (:Update
              (Transformation|SetRelativeRotation (Variables|Default|Getlever) (Math|Rotator|Lerp(Rotator) "0, 0,230.000000" "0, 0,130.000000" _newtrack_0) false false)
              (if (Variables|Default|GetIsOff)
                (bind _output_get (Variables|Default|SetPointLight (Variables|Default|GetPointLight)))
                (Rendering|Components|Light|SetLightColor _output_get "(R=0.000000,G=1.000000,B=0.069329,A=1.000000)" true)
                (Default|CallGetPowertoDoor)
                (else
                  (bind _output_get_2 (Variables|Default|SetPointLight (Variables|Default|GetPointLight)))
                  (Rendering|Components|Light|SetLightColor _output_get_2 "(R=1.000000,G=0.000000,B=0.000000,A=1.000000)" true)
                  (Default|CallCutPowertoDoor))))))
        (:B
          (Variables|Default|SetIsOff false)
          (Timeline|switching Reverse))))))

(fn ConstructionScript)

(fn Show)